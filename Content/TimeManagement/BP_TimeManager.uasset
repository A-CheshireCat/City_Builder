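; BP_TimeManager is an actor that advances an in-game time of day on a 24-hour clock, with player-switchable speeds.
; Enhanced Input actions set a Normal, Fast or Super Fast mode, and each Tick passes that mode's multiplier to UpdateCurrentTimeOfDay.
; That function adds the multiplier times TimeStep, wrapping at 24.
; The step ignores delta time, so clock speed depends on frame rate.
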(event Input|EnhancedActionEvents|EnhancedInputActionIA_TimeNormal
  (params (ActionValue :type Boolean) (ElapsedSeconds :type Float%20%28double-precision%29) (TriggeredSeconds :type Float%20%28double-precision%29) (InputAction :type Input%20Action%20Object%20Reference :default "/Game/Character/Input/IA_TimeNormal.IA_TimeNormal"))
  (:Triggered
    (Variables|Default|SetTimeModeEnum "NewEnumerator0")))

(event Input|EnhancedActionEvents|EnhancedInputActionIA_TimeFast
  (params (ActionValue :type Boolean) (ElapsedSeconds :type Float%20%28double-precision%29) (TriggeredSeconds :type Float%20%28double-precision%29) (InputAction :type Input%20Action%20Object%20Reference :default "/Game/Character/Input/IA_TimeFast.IA_TimeFast"))
  (:Triggered
    (Variables|Default|SetTimeModeEnum "NewEnumerator1")))

(event Input|EnhancedActionEvents|EnhancedInputActionIA_TimeSuperFast
  (params (ActionValue :type Boolean) (ElapsedSeconds :type Float%20%28double-precision%29) (TriggeredSeconds :type Float%20%28double-precision%29) (InputAction :type Input%20Action%20Object%20Reference :default "/Game/Character/Input/IA_TimeSuperFast.IA_TimeSuperFast"))
  (:Triggered
    (Variables|Default|SetTimeModeEnum "NewEnumerator2")))

(event EventBeginPlay
  (Input|EnableInput (Game|GetPlayerController 0)))

(event EventTick
  (params (DeltaSeconds :type Float%20%28single-precision%29))
  (switch Utilities|FlowControl|Switch|SwitchonEnum_TimeDilation (Variables|Default|GetTimeModeEnum)
    (:NewEnumerator0
      (CallFunction|UpdateCurrentTimeOfDay (Variables|Default|GetNormalSpeed)))
    (:NewEnumerator1
      (CallFunction|UpdateCurrentTimeOfDay (Variables|Default|GetFastSpeed)))
    (:NewEnumerator2
      (CallFunction|UpdateCurrentTimeOfDay (Variables|Default|GetSuperFastSpeed)))))

(fn ConstructionScript)

(fn UpdateCurrentTimeOfDay
  (params (SpeedModifier :type Float%20%28double-precision%29))
  (if (>= (+ (Variables|Default|GetCurrentTimeOfDay) (* SpeedModifier (LocalVariables|GetTimeStep))) 24.0)
    (Variables|Default|SetCurrentTimeOfDay (- (+ (Variables|Default|GetCurrentTimeOfDay) (* SpeedModifier (LocalVariables|GetTimeStep))) 24.0))
    (else
      (Variables|Default|SetCurrentTimeOfDay (+ (Variables|Default|GetCurrentTimeOfDay) (* SpeedModifier (LocalVariables|GetTimeStep)))))))