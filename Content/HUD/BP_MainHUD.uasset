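; BP_MainHUD is the HUD class that shows the main HUD widget and resolves mouse box selection of grid cells.
; On BeginPlay it creates WBP_MainHUDWidget and adds it to the viewport.
; Selection start and end events store screen positions and set a flag, which DrawHUD consumes to run GetActorsInSelectionRectangle for BP_GridCell actors.
; The results go to BP_CameraController, cast from the player character, via SelectionRectangleCallback.
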(event Custom|OnMouseSelectionStart
  (params (StartPos :type Vector%202D%20Structure))
  (Variables|Default|SetSelectionStartPos StartPos))

(event Custom|OnMouseSelectionEnd
  (params (EndPos :type Vector%202D%20Structure))
  (Variables|Default|SetSelectionEndPos EndPos)
  (Variables|Default|SetSelectionFlag true))

(event EventBeginPlay
  (bind _returnvalue (UserInterface|CreateWidget "/Game/HUD/WBP_MainHUDWidget.WBP_MainHUDWidget_C"))
  (bind _output_get (Variables|Default|SetMainHudWidgetRef _returnvalue))
  (UserInterface|Viewport|AddtoViewport _output_get 0))

(event EventDrawHUD
  (params (SizeX :type Integer) (SizeY :type Integer))
  (if (Variables|Default|GetSelectionFlag)
    (Variables|Default|SetSelectionFlag false)
    (bind _asbp_camera_controller (Utilities|Casting|CastToBP_CameraController (Game|GetPlayerCharacter 0)))
    (Default|SelectionRectangleCallback _asbp_camera_controller (Class|HUD|GetActorsinSelectionRectangle "/Game/GameObjects/Grid/BP_GridCell.BP_GridCell_C" (Variables|Default|GetSelectionStartPos) (Variables|Default|GetSelectionEndPos) true false))))

(fn ConstructionScript)