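; City builder game mode base that handles purchases against the player's money.
; CanAffordObject compares a cost with CurrentMoney on BP_GameState.
; ObjectBought reuses that check and, when it passes, subtracts the cost from CurrentMoney, otherwise doing nothing.
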(event EventBeginPlay)

(event EventTick
  (params (DeltaSeconds :type Float%20%28single-precision%29)))

(fn ConstructionScript)

(fn CanAffordObject
  (params (ObjectAmount :type Integer))
  (bind _asbp_game_state (Utilities|Casting|CastToBP_GameState (Game|GetGameState)))
  (return (<= ObjectAmount (Variables|/Game/GameModes/BP_GameState.BP_GameState_C|GetCurrentMoney _asbp_game_state))))

(fn ObjectBought
  (params (ObjectAmount :type Integer))
  (bind _canafford (CallFunction|CanAffordObject ObjectAmount))
  (if _canafford
    (bind _asbp_game_state (Utilities|Casting|CastToBP_GameState (Game|GetGameState)))
    (Variables|/Game/GameModes/BP_GameState.BP_GameState_C|SetCurrentMoney _asbp_game_state (- (Variables|/Game/GameModes/BP_GameState.BP_GameState_C|GetCurrentMoney _asbp_game_state) ObjectAmount))))