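; BP_Road is a grid-placed road tile building that adjusts its edge pathways to match neighbouring tiles.
; On BeginPlay it sets its BuildingType to the enum value it later checks neighbours against.
; When a road tile is added, OnNewRoadTileAdded checks the north, south, west and east neighbour cells.
; Each side's pathway is hidden next to a road and shown otherwise, including where no cell exists.
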(event Custom|OnNewRoadTileAdded
  (bind _gridcellref (Variables|Default|GetGridCellRef))
  (CallFunction|UpdateSideOfRoadTile (Variables|/Game/GameObjects/Grid/BP_GridCell.BP_GridCell_C|GetNeighbourN _gridcellref) (Variables|Default|GetPathway%20N))
  (CallFunction|UpdateSideOfRoadTile (Variables|/Game/GameObjects/Grid/BP_GridCell.BP_GridCell_C|GetNeighbourS _gridcellref) (Variables|Default|GetPathway%20S))
  (CallFunction|UpdateSideOfRoadTile (Variables|/Game/GameObjects/Grid/BP_GridCell.BP_GridCell_C|GetNeighbourW _gridcellref) (Variables|Default|GetPathway%20W))
  (CallFunction|UpdateSideOfRoadTile (Variables|/Game/GameObjects/Grid/BP_GridCell.BP_GridCell_C|GetNeighbourE _gridcellref) (Variables|Default|GetPathway%20E)))

(event EventBeginPlay
  (|CallParentFunction)
  (Variables|Default|SetBuildingType "NewEnumerator2"))

(event Collision|EventActorBeginOverlap
  (params (OtherActor :type Actor%20Object%20Reference))
  (|CallParentFunction OtherActor) ; This node is disabled and will not be called.\nDrag off pins to build functionality.
)

(event EventTick
  (params (DeltaSeconds :type Float%20%28single-precision%29))
  (|CallParentFunction DeltaSeconds) ; This node is disabled and will not be called.\nDrag off pins to build functionality.
)

(fn ConstructionScript
  (|CallParentFunction))

(fn UpdateSideOfRoadTile
  (params (GridCellRef :type BP%20Grid%20Cell%20Object%20Reference) (Pathway :type Static%20Mesh%20Component%20Object%20Reference))
  (Utilities|IsValid GridCellRef
    (:Is%20Valid
      (if (Utilities|Enum|Equal(Enum) (Variables|/Game/GameObjects/Grid/BP_GridCell.BP_GridCell_C|GetBuildingType GridCellRef) "NewEnumerator2")
        (Rendering|SetVisibility Pathway false false)
        (else
          (Rendering|SetVisibility Pathway true false :!label _label))))
    (:Is%20Not%20Valid
      (goto _label))))