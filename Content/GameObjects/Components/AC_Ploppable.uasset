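; Placement validator component for a city builder that shows whether its owning actor can be placed at its current location.
; Every tick it finds the closest BP_GridManager cell and marks placement invalid if that cell is occupied or the game mode reports the cost unaffordable.
; For roads, nested diagonal-neighbour checks also reject placements completing a 2x2 road block.
; The result swaps the owner's static mesh materials between valid and invalid.
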(event EventBeginPlay
  (CallFunction|UpdateState))

(event EventTick
  (params (DeltaSeconds :type Float%20%28single-precision%29))
  (CallFunction|UpdateState))

(fn UpdateState
  (bind _returnvalue (Components|GetOwner))
  (bind _returnvalue_2 (Actor|GetActorOfClass "/Game/GameObjects/Grid/BP_GridManager.BP_GridManager_C"))
  (bind _outcell (Default|GetClosestGridCell _returnvalue_2 (Transformation|GetActorLocation _returnvalue)))
  (bind _output_get (Variables|Default|SetIsPlacementValid (not (Variables|/Game/GameObjects/Grid/BP_GridCell.BP_GridCell_C|GetIsOccupied _outcell))))
  (CallFunction|RoadPlaceableCheck _outcell)
  (CallFunction|CostCheck)
  (for _array_element (Actor|GetComponentsByClass _returnvalue "/Script/Engine.StaticMeshComponent")
    (if _output_get
      (Rendering|Material|SetMaterial _array_element 0 (Variables|Default|GetMaterial))
      (else
        (Rendering|Material|SetMaterial _array_element 0 (Variables|Default|GetInvalidMaterial))))))

(fn RoadPlaceableCheck
  (params (InGridCell :type BP%20Grid%20Cell%20Object%20Reference))
  (bind _neighbourn (Variables|/Game/GameObjects/Grid/BP_GridCell.BP_GridCell_C|GetNeighbourN InGridCell))
  (bind _neighbours (Variables|/Game/GameObjects/Grid/BP_GridCell.BP_GridCell_C|GetNeighbourS InGridCell))
  (bind _neighbourw (Variables|/Game/GameObjects/Grid/BP_GridCell.BP_GridCell_C|GetNeighbourW InGridCell))
  (bind _neighboure (Variables|/Game/GameObjects/Grid/BP_GridCell.BP_GridCell_C|GetNeighbourE InGridCell))
  (bind _buildingtype (Variables|/Game/GameObjects/Grid/BP_GridCell.BP_GridCell_C|GetBuildingType _neighbourw))
  (bind _neighboure_2 (Variables|/Game/GameObjects/Grid/BP_GridCell.BP_GridCell_C|GetNeighbourE _neighbours))
  (bind _neighbourw_2 (Variables|/Game/GameObjects/Grid/BP_GridCell.BP_GridCell_C|GetNeighbourW _neighbourn))
  (bind _neighbourw_3 (Variables|/Game/GameObjects/Grid/BP_GridCell.BP_GridCell_C|GetNeighbourW _neighbours))
  (bind _neighboure_3 (Variables|/Game/GameObjects/Grid/BP_GridCell.BP_GridCell_C|GetNeighbourE _neighbourn))
  (bind _buildingtype_2 (Variables|/Game/GameObjects/Grid/BP_GridCell.BP_GridCell_C|GetBuildingType _neighbourn))
  (bind _buildingtype_3 (Variables|/Game/GameObjects/Grid/BP_GridCell.BP_GridCell_C|GetBuildingType _neighboure))
  (bind _buildingtype_4 (Variables|/Game/GameObjects/Grid/BP_GridCell.BP_GridCell_C|GetBuildingType _neighbours))
  (bind _returnvalue (Utilities|Enum|Equal(Enum) _buildingtype_2 "NewEnumerator2"))
  (bind _returnvalue_2 (Utilities|Enum|Equal(Enum) _buildingtype_4 "NewEnumerator2"))
  (bind _returnvalue_3 (Utilities|Enum|Equal(Enum) _buildingtype "NewEnumerator2"))
  (bind _returnvalue_4 (Utilities|Enum|Equal(Enum) _buildingtype_3 "NewEnumerator2"))
  (bind _asbp_placeable_actor_base (Utilities|Casting|CastToBP_PlaceableActorBase (Components|GetOwner))
    (:then
      (if (Utilities|Enum|Equal(Enum) (Variables|/Game/GameObjects/Objects/BP_PlaceableActorBase.BP_PlaceableActorBase_C|GetBuildingType _asbp_placeable_actor_base) "NewEnumerator2")
        (Utilities|IsValid _neighbourn
          (:Is%20Valid
            (Utilities|IsValid _neighbourw
              (:Is%20Valid
                ;[1 1 1] NW
                (if (and _returnvalue _returnvalue_3)
                  (Utilities|IsValid _neighbourw_2
                    (:Is%20Valid
                      (if (Utilities|Enum|Equal(Enum) (Variables|/Game/GameObjects/Grid/BP_GridCell.BP_GridCell_C|GetBuildingType _neighbourw_2) "NewEnumerator2")
                        (Variables|Default|SetIsPlacementValid false)
                        (return)
                        (else
                          _)))
                    (:Is%20Not%20Valid
                      _)))
                (Utilities|IsValid _neighboure
                  (:Is%20Valid
                    ;[1 1 1] NE
                    (if (and _returnvalue _returnvalue_4)
                      (Utilities|IsValid _neighboure_3
                        (:Is%20Valid
                          (if (Utilities|Enum|Equal(Enum) (Variables|/Game/GameObjects/Grid/BP_GridCell.BP_GridCell_C|GetBuildingType _neighboure_3) "NewEnumerator2")
                            (Variables|Default|SetIsPlacementValid false)
                            (return)
                            (else
                              _)))
                        (:Is%20Not%20Valid
                          _)))
                    (Utilities|IsValid _neighbours
                      (:Is%20Valid
                        ;[1 1 1] SE
                        (if (and _returnvalue_4 _returnvalue_2)
                          (Utilities|IsValid _neighboure_2
                            (:Is%20Valid
                              (if (Utilities|Enum|Equal(Enum) (Variables|/Game/GameObjects/Grid/BP_GridCell.BP_GridCell_C|GetBuildingType _neighboure_2) "NewEnumerator2")
                                (Variables|Default|SetIsPlacementValid false)
                                (return)
                                (else
                                  _)))
                            (:Is%20Not%20Valid
                              _)))
                        ;[1 1 1] SW
                        (if (and _returnvalue_2 _returnvalue_3)
                          (Utilities|IsValid _neighbourw_3
                            (:Is%20Valid
                              (if (Utilities|Enum|Equal(Enum) (Variables|/Game/GameObjects/Grid/BP_GridCell.BP_GridCell_C|GetBuildingType _neighbourw_3) "NewEnumerator2")
                                (Variables|Default|SetIsPlacementValid false)
                                (return)))))))))))))
        (else
          (return))))
    (:CastFailed
      (return))))

(fn CostCheck
  (bind _asbp_placeable_actor_base (Utilities|Casting|CastToBP_PlaceableActorBase (Components|GetOwner)))
  (bind _asgm_city_builder_base (Utilities|Casting|CastToGM_CityBuilderBase (Game|GetGameMode)))
  (bind _canafford (Default|CanAffordObject _asgm_city_builder_base (Variables|/Game/GameObjects/Objects/BP_PlaceableActorBase.BP_PlaceableActorBase_C|GetObjectCost _asbp_placeable_actor_base)))
  (if (not _canafford)
    (Variables|Default|SetIsPlacementValid false)))