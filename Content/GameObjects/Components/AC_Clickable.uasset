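; AC_Clickable is an actor component that makes its owner respond to cursor hover and clicks.
; On BeginPlay it binds the owner's click event and, if a static mesh is found, its cursor-over events, which toggle the mesh's custom depth rendering.
; Each click flips IsClicked and swaps the first material slot between red and green.
; InPlacementMode destroys the component, removing it from the owner.
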(event Custom|OnMouseHoverStart
  (params (TouchedActor :type Actor%20Object%20Reference))
  ;[1 1 1] OnMouseHoverStart
  (Rendering|SetRenderCustomDepth (Variables|Default|GetStaticMeshRef) true))

(event Custom|OnMouseClicked
  (params (TouchedActor :type Actor%20Object%20Reference) (ButtonPressed :type Key%20Structure :default "None"))
  (bind _staticmeshref (Variables|Default|GetStaticMeshRef))
  ;[1 1 1] OnMouseClicked
  (bind _output_get (Variables|Default|SetIsClicked (not (Variables|Default|GetIsClicked))))
  (Utilities|IsValid _staticmeshref
    (:Is%20Valid
      (if _output_get
        (Rendering|Material|SetMaterial _staticmeshref 0 "/Game/Materials/Placement/M_Red.M_Red")
        (else
          (Rendering|Material|SetMaterial _staticmeshref 0 "/Game/Materials/Placement/M_Green.M_Green"))))))

(event Custom|OnMouseHoverEnd
  (params (TouchedActor :type Actor%20Object%20Reference))
  ;[1 1 1] OnMouseHoverEnd
  (Rendering|SetRenderCustomDepth (Variables|Default|GetStaticMeshRef) false))

(event Custom|InPlacementMode
  (Components|DestroyComponent))

(event EventBeginPlay
  (bind _returnvalue (Components|GetOwner))
  (bind _returnvalue_2 (Actor|GetComponentbyClass _returnvalue "/Script/Engine.StaticMeshComponent"))
  (EventDispatchers|BindEventtoOnClicked _returnvalue (delegate Custom|OnMouseClicked))
  (Utilities|IsValid _returnvalue_2
    (:Is%20Valid
      (bind _output_get (Variables|Default|SetStaticMeshRef _returnvalue_2))
      (Rendering|SetRenderCustomDepth _output_get false)
      (EventDispatchers|BindEventtoOnBeginCursorOver _returnvalue (delegate Custom|OnMouseHoverStart))
      (EventDispatchers|BindEventtoOnEndCursorOver _returnvalue (delegate Custom|OnMouseHoverEnd)))))