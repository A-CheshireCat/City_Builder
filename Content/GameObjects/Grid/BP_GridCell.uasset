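; BP_GridCell is a grid cell actor that tracks its zoning, occupancy and building.
; SetOccupied stores the building type and reference, and SetZoneType stores the zone; both then refresh the cube's material.
; The zone material shows only for the first building-type enum value; other types get the base material.
; As a debug aid, occupying a cell turns neighbour spheres red, checked in a nested N-S-E-W chain that stops at the first invalid one.
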(event Custom|SetOccupied
  (params (OccupyingBuildingType :type Enum_BuildingType%20Enum :default "NewEnumerator0") (OccupyingBuildingRef :type Actor%20Object%20Reference))
  (bind _neighbourn (Variables|Default|GetNeighbourN))
  (bind _neighbours (Variables|Default|GetNeighbourS))
  (bind _neighboure (Variables|Default|GetNeighbourE))
  (bind _neighbourw (Variables|Default|GetNeighbourW))
  (Variables|Default|SetIsOccupied true)
  (Variables|Default|SetBuildingType OccupyingBuildingType)
  (Variables|Default|SetBuildingRef OccupyingBuildingRef)
  (CallFunction|UpdateZoningRepresentation)
  ;[1 1 1] Debug Neighbours
  (Utilities|IsValid _neighbourn
    (:Is%20Valid
      (CallFunction|DebugShowNeigborOccupied _neighbourn)
      (Utilities|IsValid _neighbours
        (:Is%20Valid
          (CallFunction|DebugShowNeigborOccupied _neighbours)
          (Utilities|IsValid _neighboure
            (:Is%20Valid
              (CallFunction|DebugShowNeigborOccupied _neighboure)
              (Utilities|IsValid _neighbourw
                (:Is%20Valid
                  (CallFunction|DebugShowNeigborOccupied _neighbourw))))))))))

(event Custom|DebugShowNeigborOccupied
  (Rendering|Material|SetMaterial (Variables|Default|GetSphere) 0 "/Game/Materials/Placement/M_Red.M_Red"))

(event Custom|SetZoneType
  (params (Zone :type Enum_ZoningType%20Enum :default "NewEnumerator0"))
  (Variables|Default|SetZoningType Zone)
  (CallFunction|UpdateZoningRepresentation))

(event EventBeginPlay)

(event Collision|EventActorBeginOverlap
  (params (OtherActor :type Actor%20Object%20Reference)))

(event EventTick
  (params (DeltaSeconds :type Float%20%28single-precision%29)))

(fn ConstructionScript)

(fn UpdateZoningRepresentation
  (if (Utilities|Enum|Equal(Enum) (Variables|Default|GetBuildingType) "NewEnumerator0")
    (switch Utilities|FlowControl|Switch|SwitchonEnum_ZoningType (Variables|Default|GetZoningType)
      (:NewEnumerator0
        (Rendering|Material|SetMaterial (Variables|Default|GetCube) 0 "/Game/Materials/Zones/MI_ZoneResidential.MI_ZoneResidential"))
      (:NewEnumerator1
        (Rendering|Material|SetMaterial (Variables|Default|GetCube) 0 "/Game/Materials/Zones/MI_ZoneCommercial.MI_ZoneCommercial"))
      (:NewEnumerator2
        (Rendering|Material|SetMaterial (Variables|Default|GetCube) 0 "/Game/Materials/Zones/MI_ZoneIndustrial.MI_ZoneIndustrial")))
    (else
      (Rendering|Material|SetMaterial (Variables|Default|GetCube) 0 "/Game/Materials/Zones/M_ZoneBase.M_ZoneBase"))))